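; BP_MovableObjects is a movable object actor that can appear as either a 3D static mesh or a 2D Paper sprite.
; The construction script applies the mesh if valid, otherwise the sprite if valid, setting the Is3D flag to match.
; On BeginPlay, after calling the parent, it sets both components to block or ignore the Pawn collision channel based on ShouldBlockCharacter.
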(event `self.ReceiveBeginPlay`
  (bind _staticmesh (`self.StaticMesh`))
  (`parent.ReceiveBeginPlay`)
  (if (`self.ShouldBlockCharacter?`)
    (`PrimitiveComponent.SetCollisionResponseToChannel` _staticmesh "ECC_Pawn" "ECR_Block")
    (`PrimitiveComponent.SetCollisionResponseToChannel` (`self.PaperSprite`) "ECC_Pawn" "ECR_Block")
    (else
      (`PrimitiveComponent.SetCollisionResponseToChannel` _staticmesh "ECC_Pawn" "ECR_Ignore")
      (`PrimitiveComponent.SetCollisionResponseToChannel` (`self.PaperSprite`) "ECC_Pawn" "ECR_Ignore"))))

(fn `UserConstructionScript`
  (`/Engine/EditorBlueprintResources/StandardMacros.IsValid` (`self.Moveable3DObject`)
    (:`Is Valid`
      (`StaticMeshComponent.SetStaticMesh` (`self.StaticMesh`) (`self.Moveable3DObject`))
      (set `self.Is3D?` true))
    (:`Is Not Valid`
      (`/Engine/EditorBlueprintResources/StandardMacros.IsValid` (`self.Moveable2DSprite`)
        (:`Is Valid`
          (`PaperSpriteComponent.SetSprite` (`self.PaperSprite`) (`self.Moveable2DSprite`))
          (set `self.Is3D?` false))))))