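; BP_FollowCamera is a camera Blueprint that follows a sprite-based target, Cible, in a side-view plane.
; Each Tick it interpolates its scene component toward the target sprite's X and Z while keeping its own Y fixed.
; It switches to a separate interpolation speed when the target falls faster than a set threshold, so long drops are tracked differently.
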(event `self.ReceiveTick`
  (params (DeltaSeconds :type "Float (single-precision)"))
  (bind _cible (`self.Cible`))
  (bind _returnvalue (`SceneComponent.K2_GetComponentLocation` (`self.SceneComponent`)))
  ;[1 1 1] Interpolate to player position
  (`/Engine/EditorBlueprintResources/StandardMacros.IsValid` _cible
    (:`Is Valid`
      (`SceneComponent.K2_SetWorldLocation` (`self.SceneComponent`) (`KismetMathLibrary.VInterpTo` _returnvalue (`KismetMathLibrary.MakeVector` (.x (`SceneComponent.K2_GetComponentLocation` (`PaperCharacter.Sprite` _cible))) (.y _returnvalue) (.z (`SceneComponent.K2_GetComponentLocation` (`PaperCharacter.Sprite` _cible)))) DeltaSeconds (select `bool` (<= (.z (`self.GetVelocity` (`self.Cible`))) -1500.0) :`false` (`self.NormalInterpolationSpeed`) :`true` (`self.BigFallInterpolationSpeed`))) false false))))

(fn `UserConstructionScript`)