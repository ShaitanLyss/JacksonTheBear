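; BP_MasterFallingObj is an environment actor, named as a master for falling objects, that shows a configurable texture on a Plane.
; The construction script creates a dynamic material instance and feeds TextureOfTheObject into its BGLayerTexture parameter.
; It hides the plane when no texture is valid and scales it by ObjectScale times SIze.
; The event graph holds only disabled stubs, so no falling movement is implemented here.
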(fn `UserConstructionScript`
  (bind _plane (`self.Plane`))
  (bind _textureoftheobject (`self.TextureOfTheObject`))
  (bind _plane_2 (`self.Plane`))
  (bind _returnvalue (`PrimitiveComponent.CreateDynamicMaterialInstance` _plane 0 (`PrimitiveComponent.GetMaterial` _plane 0) "None"))
  (bind _output_get (set `self.Mat` _returnvalue))
  (`PrimitiveComponent.SetMaterial` _plane 0 _output_get)
  (`MaterialInstanceDynamic.SetTextureParameterValue` (`self.Mat`) "BGLayerTexture" _textureoftheobject)
  (`/Engine/EditorBlueprintResources/StandardMacros.IsValid` _textureoftheobject
    (:`Is Valid`
      (`SceneComponent.SetVisibility` _plane_2 true false))
    (:`Is Not Valid`
      (`SceneComponent.SetVisibility` _plane_2 false false)))
  (`SceneComponent.SetRelativeScale3D` _plane (* (`self.ObjectScale`) (`self.SIze`))))