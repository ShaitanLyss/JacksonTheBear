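; A one-shot trigger actor that drops a random falling object when the 2D side-scroller character enters its trigger box.
; On overlap it spawns a random class from its object array at the SpawnPoint transform, passing in size and texture.
; A Done flag then blocks further spawns.
; The construction script offsets SpawnPoint by FallPointLocation to position the drop.
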(event `FallObject`
  (bind _objectthatwillfall (`self.ObjectThatWIllFall`))
  (if (`self.Done?`)
    _
    (elif (`KismetArrayLibrary.Array_IsValidIndex` _objectthatwillfall)
      (`|SpawnActorFromClass` (`|GetArrayItem` _objectthatwillfall (`KismetMathLibrary.RandomIntegerInRange` 0 (`KismetArrayLibrary.Array_LastIndex` _objectthatwillfall))) (`SceneComponent.K2_GetComponentToWorld` (`self.SpawnPoint`)) "AlwaysSpawn" "OverrideRootScale" null (`self.Size`) (`self.TextureOfObject`) null))))

(event `self.TriggerBox.OnComponentBeginOverlap`
  (params (OverlappedComponent :type "PrimitiveComponent Object Reference") (OtherActor :type "Actor Object Reference") (OtherComp :type "PrimitiveComponent Object Reference") (OtherBodyIndex :type Integer) (bFromSweep :type Boolean) (SweepResult :type "HitResult Structure (by ref)"))
  (cast `/Game/2DSideScrollerBP/Blueprints/2DSideScrollerCharacter` OtherActor)
  (`self.FallObject`)
  (set `self.Done?` true))

(fn `UserConstructionScript`
  (bind _spawnpoint (`self.SpawnPoint`))
  (`SceneComponent.K2_SetRelativeLocation` _spawnpoint (+ (`SceneComponent.RelativeLocation` _spawnpoint) (`self.FallPointLocation`)) false false))