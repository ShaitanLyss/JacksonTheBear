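; BP_BG is a configurable five-layer environment background, with per-layer texture, speed, tiling, offset and scale.
; The Construction Script creates a dynamic material instance per layer and sets its Speed (red channel only), Tile and BGLayerTexture parameters.
; Layers without a valid texture are hidden.
; Each layer's offset is added to its current relative location, while scale is replaced and rotation kept.
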(fn `UserConstructionScript`
  (bind _layer2 (`self.Layer2`))
  (bind _layer3 (`self.Layer3`))
  (bind _layer1 (`self.Layer1`))
  (bind _layer2mat (`self.Layer2Mat`))
  (bind _layer2texture (`self.Layer2Texture`))
  (bind _layer5texture (`self.Layer5Texture`))
  (bind _layer3mat (`self.Layer3Mat`))
  (bind _layer3texture (`self.Layer3Texture`))
  (bind _layer4mat (`self.Layer4Mat`))
  (bind _layer4 (`self.Layer4`))
  (bind _layer4texture (`self.Layer4Texture`))
  (bind _layer5 (`self.Layer5`))
  (bind _layer2_2 (`self.Layer2`))
  (bind _layer3_2 (`self.Layer3`))
  (bind _layer4_2 (`self.Layer4`))
  (bind _layer5_2 (`self.Layer5`))
  (bind _layer1_2 (`self.Layer1`))
  (bind _layer2_3 (`self.Layer2`))
  (bind _layer3_3 (`self.Layer3`))
  (bind _layer4_3 (`self.Layer4`))
  (bind _layer5_3 (`self.Layer5`))
  (bind _layer1_3 (`self.Layer1`))
  (bind _layer5mat (`self.Layer5Mat`))
  (bind _layer1mat (`self.Layer1Mat`))
  (bind _layer1texture (`self.Layer1Texture`))
  (bind _returnvalue (`PrimitiveComponent.CreateDynamicMaterialInstance` _layer1_2 0 (`PrimitiveComponent.GetMaterial` _layer1_2 0) "None"))
  (set `self.Layer1Mat` _returnvalue)
  (`PrimitiveComponent.SetMaterial` _layer1_2 0 _returnvalue)
  (`MaterialInstanceDynamic.SetVectorParameterValue` _layer1mat "Speed" (make `LinearColor` (`self.Layer1Speed`) 0.0 0.0 1.0))
  (`MaterialInstanceDynamic.SetScalarParameterValue` _layer1mat "Tile" (`self.Layer1Tile`))
  (`MaterialInstanceDynamic.SetTextureParameterValue` _layer1mat "BGLayerTexture" _layer1texture)
  (`/Engine/EditorBlueprintResources/StandardMacros.IsValid` _layer1texture
    (:`Is Valid`
      (`SceneComponent.SetVisibility` _layer1 true false))
    (:`Is Not Valid`
      (`SceneComponent.SetVisibility` _layer1 false false)))
  (bind _returnvalue_2 (`PrimitiveComponent.CreateDynamicMaterialInstance` _layer2 0 (`PrimitiveComponent.GetMaterial` _layer2 0) "None"))
  (set `self.Layer2Mat` _returnvalue_2)
  (`PrimitiveComponent.SetMaterial` _layer2 0 _returnvalue_2)
  (`MaterialInstanceDynamic.SetVectorParameterValue` _layer2mat "Speed" (make `LinearColor` (`self.Layer2Speed`) 0.0 0.0 1.0))
  (`MaterialInstanceDynamic.SetScalarParameterValue` _layer2mat "Tile" (`self.Layer2Tile`))
  (`MaterialInstanceDynamic.SetTextureParameterValue` _layer2mat "BGLayerTexture" _layer2texture)
  (`/Engine/EditorBlueprintResources/StandardMacros.IsValid` _layer2texture
    (:`Is Valid`
      (`SceneComponent.SetVisibility` _layer2_2 true false))
    (:`Is Not Valid`
      (`SceneComponent.SetVisibility` _layer2_2 false false)))
  (bind _returnvalue_3 (`PrimitiveComponent.CreateDynamicMaterialInstance` _layer3 0 (`PrimitiveComponent.GetMaterial` _layer3 0) "None"))
  (set `self.Layer3Mat` _returnvalue_3)
  (`PrimitiveComponent.SetMaterial` _layer3 0 _returnvalue_3)
  (`MaterialInstanceDynamic.SetVectorParameterValue` _layer3mat "Speed" (make `LinearColor` (`self.Layer3Speed`) 0.0 0.0 1.0))
  (`MaterialInstanceDynamic.SetScalarParameterValue` _layer3mat "Tile" (`self.Layer3Tile`))
  (`MaterialInstanceDynamic.SetTextureParameterValue` _layer3mat "BGLayerTexture" _layer3texture)
  (`/Engine/EditorBlueprintResources/StandardMacros.IsValid` _layer3texture
    (:`Is Valid`
      (`SceneComponent.SetVisibility` _layer3_2 true false))
    (:`Is Not Valid`
      (`SceneComponent.SetVisibility` _layer3_2 false false)))
  (bind _returnvalue_4 (`PrimitiveComponent.CreateDynamicMaterialInstance` _layer4 0 (`PrimitiveComponent.GetMaterial` _layer4 0) "None"))
  (set `self.Layer4Mat` _returnvalue_4)
  (`PrimitiveComponent.SetMaterial` _layer4 0 _returnvalue_4)
  (`MaterialInstanceDynamic.SetVectorParameterValue` _layer4mat "Speed" (make `LinearColor` (`self.Layer4Speed`) 0.0 0.0 1.0))
  (`MaterialInstanceDynamic.SetScalarParameterValue` _layer4mat "Tile" (`self.Layer4Tile`))
  (`MaterialInstanceDynamic.SetTextureParameterValue` _layer4mat "BGLayerTexture" _layer4texture)
  (`/Engine/EditorBlueprintResources/StandardMacros.IsValid` _layer4texture
    (:`Is Valid`
      (`SceneComponent.SetVisibility` _layer4_2 true false))
    (:`Is Not Valid`
      (`SceneComponent.SetVisibility` _layer4_2 false false)))
  (bind _returnvalue_5 (`PrimitiveComponent.CreateDynamicMaterialInstance` _layer5_2 0 (`PrimitiveComponent.GetMaterial` _layer5_2 0) "None"))
  (set `self.Layer5Mat` _returnvalue_5)
  (`PrimitiveComponent.SetMaterial` _layer5_2 0 _returnvalue_5)
  (`MaterialInstanceDynamic.SetVectorParameterValue` _layer5mat "Speed" (make `LinearColor` (`self.Layer5Speed`) 0.0 0.0 1.0))
  (`MaterialInstanceDynamic.SetScalarParameterValue` _layer5mat "Tile" (`self.Layer5Tile`))
  (`MaterialInstanceDynamic.SetTextureParameterValue` _layer5mat "BGLayerTexture" _layer5texture)
  (`/Engine/EditorBlueprintResources/StandardMacros.IsValid` _layer5texture
    (:`Is Valid`
      (`SceneComponent.SetVisibility` _layer5 true false))
    (:`Is Not Valid`
      (`SceneComponent.SetVisibility` _layer5 false false)))
  (`SceneComponent.K2_SetRelativeTransform` _layer1_3 (`KismetMathLibrary.MakeTransform` (+ (`SceneComponent.RelativeLocation` _layer1_3) (`self.Layer1Location`)) (`SceneComponent.RelativeRotation` _layer1_3) (`self.Layer1Scale`)) false false)
  (`SceneComponent.K2_SetRelativeTransform` _layer2_3 (`KismetMathLibrary.MakeTransform` (+ (`SceneComponent.RelativeLocation` _layer2_3) (`self.Layer2Location`)) (`SceneComponent.RelativeRotation` _layer2_3) (`self.Layer2Scale`)) false false)
  (`SceneComponent.K2_SetRelativeTransform` _layer3_3 (`KismetMathLibrary.MakeTransform` (+ (`SceneComponent.RelativeLocation` _layer3_3) (`self.Layer3Location`)) (`SceneComponent.RelativeRotation` _layer3_3) (`self.Layer3Scale`)) false false)
  (`SceneComponent.K2_SetRelativeTransform` _layer4_3 (`KismetMathLibrary.MakeTransform` (+ (`SceneComponent.RelativeLocation` _layer4_3) (`self.Layer4Location`)) (`SceneComponent.RelativeRotation` _layer4_3) (`self.Layer4Scale`)) false false)
  (`SceneComponent.K2_SetRelativeTransform` _layer5_3 (`KismetMathLibrary.MakeTransform` (+ (`SceneComponent.RelativeLocation` _layer5_3) (`self.Layer5Location`)) (`SceneComponent.RelativeRotation` _layer5_3) (`self.Layer5Scale`)) false false))