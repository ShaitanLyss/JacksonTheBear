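; BP_PlantTree is an interactable tree-planting spot that changes appearance when a tree is planted.
; The construction script shows the initial mesh, and OnTreePlant starts green smoke, then swaps to the second mesh after a delay.
; After another delay it stops the smoke, clears the referenced character's interaction flag, calls ToggleMovement to restore movement and sets ShowWidget to false.
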(event `OnTreePlant`
  (bind _charref (`self.CharRef`))
  (`ActorComponent.Activate` (`self.P_GreenSmoke`) false)
  (`KismetSystemLibrary.Delay` 4.0)
  (`StaticMeshComponent.SetStaticMesh` (`self.Mesh`) (`self.Mesh2`))
  (`KismetSystemLibrary.Delay` 2.0)
  (`ActorComponent.Deactivate` (`self.P_GreenSmoke`))
  (set `/Game/2DSideScrollerBP/Blueprints/2DSideScrollerCharacter.AlreadyInteracting?` false _charref)
  (`/Game/2DSideScrollerBP/Blueprints/2DSideScrollerCharacter.ToggleMovement` _charref true)
  (set `self.ShowWidget?` false))

(fn `UserConstructionScript`
  (`parent.UserConstructionScript`)
  (`StaticMeshComponent.SetStaticMesh` (`self.Mesh`) (`self.Mesh1`)))