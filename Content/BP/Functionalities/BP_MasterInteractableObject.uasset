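; Base interactable object for the side-scroller character, showing an animated prompt when the character is nearby.
; On BeginPlay it fills the widget with its name, interaction text and icon.
; Box overlap registers it as the character's InteractableObject if ShowWidget is set and the character is not already interacting.
; Leaving plays the hide animation before hiding the widget, clearing that reference unless an interaction is underway.
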(event `self.ReceiveBeginPlay`
  (set `self.InteractionWidget` (cast `/Game/Widgets/InteractionWidget` (`WidgetComponent.GetUserWidgetObject` (`self.Widget`)) :!pure true))
  (`self.InItWidget`))

(event `self.Box.OnComponentBeginOverlap`
  (params (OverlappedComponent :type "PrimitiveComponent Object Reference") (OtherActor :type "Actor Object Reference") (OtherComp :type "PrimitiveComponent Object Reference") (OtherBodyIndex :type Integer) (bFromSweep :type Boolean) (SweepResult :type "HitResult Structure (by ref)"))
  (if (`self.ShowWidget?`)
    (bind _as2dside_scroller_character (cast `/Game/2DSideScrollerBP/Blueprints/2DSideScrollerCharacter` OtherActor))
    (if (not (`/Game/2DSideScrollerBP/Blueprints/2DSideScrollerCharacter.AlreadyInteracting?` _as2dside_scroller_character))
      (set `self.CharRef` _as2dside_scroller_character)
      (set `/Game/2DSideScrollerBP/Blueprints/2DSideScrollerCharacter.InteractableObject` self _as2dside_scroller_character)
      (`SceneComponent.SetVisibility` (`self.Widget`) true false)
      (`/Game/Widgets/InteractionWidget.PlayAnim` (`self.InteractionWidget`) false))))

(event `HideWidget`
  (`/Game/Widgets/InteractionWidget.PlayAnim` (`self.InteractionWidget`) true)
  (`KismetSystemLibrary.Delay` 1.0)
  (`SceneComponent.SetVisibility` (`self.Widget`) false false))

(event `self.Box.OnComponentEndOverlap`
  (params (OverlappedComponent :type "PrimitiveComponent Object Reference") (OtherActor :type "Actor Object Reference") (OtherComp :type "PrimitiveComponent Object Reference") (OtherBodyIndex :type Integer))
  (bind _as2dside_scroller_character (cast `/Game/2DSideScrollerBP/Blueprints/2DSideScrollerCharacter` OtherActor))
  (if (`/Game/2DSideScrollerBP/Blueprints/2DSideScrollerCharacter.AlreadyInteracting?` _as2dside_scroller_character)
    (`self.HideWidget`)
    (else
      (set `/Game/2DSideScrollerBP/Blueprints/2DSideScrollerCharacter.InteractableObject` null _as2dside_scroller_character)
      (`self.HideWidget`))))

(fn `InItWidget`
  (bind _interactionwidget (`self.InteractionWidget`))
  (`TextBlock.SetText` (`/Game/Widgets/InteractionWidget.NameText` _interactionwidget) (`self.NameText`))
  (`TextBlock.SetText` (`/Game/Widgets/InteractionWidget.InteractionText` _interactionwidget) (`self.InteractionText`))
  (`Image.SetBrushFromTexture` (`/Game/Widgets/InteractionWidget.Icon` _interactionwidget) (`self.Icon`) false))

(fn `UserConstructionScript`)